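; Actor component that shows the stage-clear screen, creating the WBP_ClearStageMain widget on BeginPlay and turning on the mouse cursor.
; It fills the widget from two initial sets, passing each reward item and card through AddRewardItem and AddCard events.
; It binds the widget's exit dispatcher to ExitClearStage, which is a placeholder that only prints a debug message.
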(event Custom|AddRewardItem
  (params (FRewardItem :type F%20Clear%20Stage%20Reward%20Item%20Structure))
  (Default|AddReward (Variables|Default|GetClearStageMain) FRewardItem))

(event Custom|SetInitialRewardItem
  (for _array_element (Variables|Default|GetFRewardItemInitialSet)
    (CallFunction|AddRewardItem _array_element)))

(event Custom|ExitClearStage
  (Development|PrintString "Exit処理！！！！"))

(event Custom|AddCard
  (params (CardInfo :type F%20Clear%20Stage%20Card%20Info%20Structure))
  (Default|AddCard (Variables|Default|GetClearStageMain) CardInfo))

(event Custom|SetInitialCardSet
  (for _array_element (Variables|Default|GetCardInfoInitialSet)
    (CallFunction|AddCard _array_element)
    (Development|PrintString "Hello")))

(event EventBeginPlay
  (Utilities|FlowControl|Sequence
    (:then_0
      (bind _returnvalue (UserInterface|CreateWidget "/Game/UIs/WBP_ClearStageMain.WBP_ClearStageMain_C"))
      (bind _output_get (Variables|Default|SetClearStageMain _returnvalue))
      (UserInterface|Viewport|AddtoViewport _output_get 0)
      (CallFunction|SetInitialRewardItem)
      (EventDispatchers|BindEventtoEDExitClearStage (Variables|Default|GetClearStageMain) (delegate Custom|ExitClearStage))
      (CallFunction|SetInitialCardSet))
    (:then_1
      (Variables|/Script/Engine.PlayerController|SetbShowMouseCursor (Game|GetPlayerController 0) true))))