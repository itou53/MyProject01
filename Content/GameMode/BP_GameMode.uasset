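; BP_GameMode is a game mode that opens a starting UI screen at BeginPlay.
; A switch on the StartPage value of DebugInfo creates either the clear-stage main widget or the card selection panel and adds it to the viewport.
; Only the main widget is stored in a variable.
; It then shows the mouse cursor on the first player controller.
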(event EventBeginPlay
  (Utilities|FlowControl|Sequence
    (:then_0
      (switch Utilities|FlowControl|Switch|SwitchonEnum_DebugInfo_StartPage (Utilities|Struct|BreakDebugInfo (Variables|Default|GetDebugInfo))
        (:NewEnumerator0
          (bind _returnvalue (UserInterface|CreateWidget "/Game/UI/W_ClearStageMain.W_ClearStageMain_C"))
          (bind _output_get (Variables|Default|SetW_ClearStageMain _returnvalue))
          (UserInterface|Viewport|AddtoViewport _output_get 0))
        (:NewEnumerator1
          (bind _returnvalue_2 (UserInterface|CreateWidget "/Game/UI/W_ClearStage_SelectCardPanel.W_ClearStage_SelectCardPanel_C"))
          (UserInterface|Viewport|AddtoViewport _returnvalue_2 0))))
    (:then_1
      (Variables|/Script/Engine.PlayerController|SetbShowMouseCursor (Game|GetPlayerController 0) true))))

(fn ConstructionScript)